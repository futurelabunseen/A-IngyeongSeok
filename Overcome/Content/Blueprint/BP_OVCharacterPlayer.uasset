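; Player character Blueprint that handles grenade throwing, gun firing and a targeting UI.
; Grenade input drives throw montages, spawns and launches BP_Grenade, and redraws a predicted spline-mesh path each frame through a self-recalling Delay loop.
; F toggles the child-actor gun between hand and back sockets, and right mouse shows the target widget.
; Left mouse, when IsAiming is set, sends FireMessage with a camera line-trace target.
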(event Custom|ShowProjectilePath
  (bind _spline_mesh_components (Variables|Default|GetSpline%20Mesh%20Components))
  (bind _projectile_path (Variables|Default|GetProjectile%20Path))
  (bind _projectile_hit (Variables|Default|Getprojectile_hit))
  ;[1 1 1] Path
  (Spline|ClearSplinePoints (Variables|Default|GetProjectile%20Path) true)
  (for _array_element _spline_mesh_components
    (Components|DestroyComponent _array_element))
  (Utilities|Array|Clear _spline_mesh_components)
  (if (Variables|Default|GetIs%20Throwing)
    (bind (_outhit _outpathpositions) (Class|GameplayStatics|BlueprintPredictProjectilePathbyTraceChannel (Transformation|GetWorldLocation (Variables|Default|GetItem%20Start)) (* (+ (Math|Vector|GetForwardVector (Pawn|GetControlRotation :!class /Script/Engine.Pawn)) "0.000000,0.000000,0.400000") 1.5e+03) true 0.0 "ECC_Camera" false (Utilities|Array|MakeArray self) "None"))
    (Transformation|SetWorldLocation _projectile_hit (.Location (Collision|BreakHitResult _outhit)) false false)
    (Rendering|SetVisibility _projectile_hit true false)
    (for (_array_element_2 _array_index) _outpathpositions
      (Spline|AddSplinePointatIndex (Variables|Default|GetProjectile%20Path) _array_element_2 _array_index "Local" true))
    (for _index (range 0 (- (Spline|GetNumberOfSplinePoints (Variables|Default|GetProjectile%20Path)) 2))
      (bind _returnvalue (AddComponent|AddSplineMeshComponent true))
      (SplineMesh|SetStartandEnd _returnvalue (Spline|GetLocationatSplinePoint _projectile_path _index "Local") (Spline|GetTangentatSplinePoint _projectile_path _index "Local") (Spline|GetLocationatSplinePoint _projectile_path _index "Local") (Spline|GetTangentatSplinePoint _projectile_path _index "Local") true :!class /Script/Engine.SplineMeshComponent)
      (Utilities|Array|Add (Variables|Default|GetSpline%20Mesh%20Components) _returnvalue))
    (Utilities|FlowControl|Delay (Utilities|Time|GetWorldDeltaSeconds))
    (CallFunction|ShowProjectilePath)
    (else
      (Rendering|SetVisibility (Variables|Default|Getprojectile_hit) false false))))

(event Input|EnhancedActionEvents|EnhancedInputActionIA_OV_Grenade
  (params (ActionValue :type Boolean) (ElapsedSeconds :type Float%20%28double-precision%29) (TriggeredSeconds :type Float%20%28double-precision%29) (InputAction :type Input%20Action%20Object%20Reference :default "/Game/Input/Actions/IA_OV_Grenade.IA_OV_Grenade"))
  ;[1 1 1] Grenade
  (:Triggered
    (Animation|Montage|PlayMontage (Variables|Character|GetMesh) "/Game/Asset/Animation/AM_ThrowStart.AM_ThrowStart"
      (:then
        (if (Variables|Default|GetIs%20Spawn)
          _
          (else
            (bind _returnvalue (Game|SpawnActorfromClass "/Game/Blueprint/BP_Grenade.BP_Grenade_C" (Math|Transform|MakeTransform (Transformation|GetSocketLocation (Variables|Character|GetMesh) "Rifle_Socket") "0, 0, 0" "1.000000,1.000000,1.000000") "AlwaysSpawn" "MultiplyWithRoot" 0 0))
            (Variables|Default|SetIs%20Spawn true)
            (bind _output_get (Variables|Default|SetBP_Grenade _returnvalue))))
        (Transformation|AttachComponentToComponent _output_get (Variables|Character|GetMesh) "Item_Socket" "SnapToTarget" "SnapToTarget" "SnapToTarget" true))
      (:OnNotifyBegin
        (Variables|Default|SetIs%20Throwing true)
        (CallFunction|ShowProjectilePath))))
  (:Completed
    (if (Variables|Default|GetIs%20Throwing)
      (Animation|Montage|PlayMontage (Variables|Character|GetMesh) "/Game/Asset/Animation/AM_Throwing.AM_Throwing" 1.0 0.0 ""
        (:then
          (Variables|Default|SetIs%20Throwing false)
          (Utilities|FlowControl|Delay 0.2)
          (Utilities|IsValid (Variables|Default|GetBP_Grenade)
            (:Is%20Valid
              (Default|Throw (Variables|Default|GetBP_Grenade) (* (+ (Math|Vector|GetForwardVector (Pawn|GetControlRotation :!class /Script/Engine.Pawn)) "0.000000,0.000000,0.400000") 1.5e+03))
              (Variables|Default|SetIs%20Spawn false)))))
      (else
        (Animation|StopAnimMontage 0)))))

(event EventBeginPlay
  (bind _returnvalue (UserInterface|CreateWidget "/Game/UMG/TargetUI.TargetUI_C" 0 self))
  (bind _output_get (Variables|Default|SetUI _returnvalue))
  (UserInterface|Viewport|AddtoViewport _output_get 0)
  (Widget|SetVisibility (Variables|Default|GetUI) "Hidden"))

(event Collision|EventActorBeginOverlap
  (params (OtherActor :type Actor%20Object%20Reference)))

(event EventTick
  (params (DeltaSeconds :type Float%20%28single-precision%29)))

(event Input|MouseEvents|RightMouseButton
  (params (Key :type Key%20Structure :default "None"))
  (:Pressed
    (Widget|SetVisibility (Variables|Default|GetUI) "Visible"))
  (:Released
    (Widget|SetVisibility (Variables|Default|GetUI) "Hidden")))

(event Input|KeyboardEvents|F
  (params (Key :type Key%20Structure :default "None"))
  (:Pressed
    (Utilities|FlowControl|FlipFlop
      (:A
        (Transformation|AttachComponentToComponent (Variables|/Script/Engine.ChildActorComponent|GetChildActor (Variables|Default|GetBP_Gun)) (Variables|Character|GetMesh) "Rifle_Socket" "KeepRelative" "KeepRelative" "KeepRelative" true))
      (:B
        (Transformation|AttachComponentToComponent (Variables|/Script/Engine.ChildActorComponent|GetChildActor (Variables|Default|GetBP_Gun)) (Variables|Character|GetMesh) "Back_Socket" "KeepRelative" "KeepRelative" "KeepRelative" true)))))

(event Input|MouseEvents|LeftMouseButton
  (params (Key :type Key%20Structure :default "None"))
  ;[1 1 1] Gun
  (:Pressed
    (if (Variables|Default|GetbIsAiming)
      (Class|BPIFire|Fire(Message) (Variables|/Script/Engine.ChildActorComponent|GetChildActor (Variables|Default|GetBP_Gun)) true (CallFunction|GetTargetLocation))))
  (:Released
    (Class|BPIFire|Fire(Message) (Variables|/Script/Engine.ChildActorComponent|GetChildActor (Variables|Default|GetBP_Gun)) false "0, 0, 0")))

(fn ConstructionScript)

(fn GetTargetLocation
  (bind _followcamera (Variables|Default|GetFollowCamera))
  (bind _returnvalue (Transformation|GetSocketLocation _followcamera "None"))
  (bind _outhit (Collision|LineTraceByChannel _returnvalue (+ _returnvalue (* (Math|Vector|GetForwardVector (Pawn|GetControlRotation (Game|GetPlayerController 0) :!class /Script/Engine.Controller)) 1e+09)) "TraceTypeQuery1" false 0 "None"))
  (return (.ImpactPoint (Collision|BreakHitResult _outhit))))