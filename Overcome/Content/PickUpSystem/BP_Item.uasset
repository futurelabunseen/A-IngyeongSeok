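; BP_Item is a pickup item actor that shrinks away and is destroyed when its PickUp event fires.
; The construction script applies the chosen mesh variable to the ItemModel component.
; PickUp plays a timeline that scales the model from full size toward zero.
; The timeline's Update pin also drives the Delay before DestroyActor, so destruction follows 0.4 seconds after the first update, independent of the timeline finishing.
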(event EventBeginPlay)

(event Collision|EventActorBeginOverlap
  (params (OtherActor :type Actor%20Object%20Reference)))

(event EventTick
  (params (DeltaSeconds :type Float%20%28single-precision%29)))

(event EventPickUp
  (bind _shrinktimeline (Timeline|Timeline Play)
    (:Update
      (Transformation|SetWorldScale3D (Variables|Default|GetItemModel) (Math|Conversions|ToVector(Float) (Math|Float|Lerp 1.0 0.0 _shrinktimeline)))
      (Utilities|FlowControl|Delay 0.4)
      (Actor|DestroyActor))))

(fn ConstructionScript
  (Components|StaticMesh|SetStaticMesh (Variables|Default|GetItemModel) (Variables|Default|GetITemModelToPlace)))